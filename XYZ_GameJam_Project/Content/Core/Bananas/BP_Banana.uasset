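; BP_Banana is a pickup that gives the overlapping BP_TopDownCharacter a random buff paired with a random debuff, then destroys itself.
; Sphere overlap rolls a weighted rarity tier (legendary, common or epic), and ApplyEffect receives one random entry from that tier's buff and debuff lists.
; While IsAttrached is set, Tick interpolates the banana toward player 0's character like a magnet.
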(event `self.Sphere.OnComponentBeginOverlap`
  (params (OverlappedComponent :type "PrimitiveComponent Object Reference") (OtherActor :type "Actor Object Reference") (OtherComp :type "PrimitiveComponent Object Reference") (OtherBodyIndex :type Integer) (bFromSweep :type Boolean) (SweepResult :type "HitResult Structure (by ref)"))
  (bind _returnvalue (`KismetMathLibrary.RandomIntegerInRange` 0 99))
  (if (>= _returnvalue 90)
    (bind _asbp_top_down_character (cast `/Game/Core/Characters/BP_TopDownCharacter` OtherActor))
    (`/Game/Core/Characters/BP_TopDownCharacter.ApplyEffect` _asbp_top_down_character (`KismetArrayLibrary.Array_Random` (`self.LegendaryBuffs`)) (`KismetArrayLibrary.Array_Random` (`self.LegendaryDebuffs`)))
    (`self.K2_DestroyActor`)
    (elif (<= _returnvalue 60)
      (bind _asbp_top_down_character_2 (cast `/Game/Core/Characters/BP_TopDownCharacter` OtherActor))
      (`/Game/Core/Characters/BP_TopDownCharacter.ApplyEffect` _asbp_top_down_character_2 (`KismetArrayLibrary.Array_Random` (`self.CommonBuffs`)) (`KismetArrayLibrary.Array_Random` (`self.CommonDebuffs`)))
      (`self.K2_DestroyActor`)
      (else
        (bind _asbp_top_down_character_3 (cast `/Game/Core/Characters/BP_TopDownCharacter` OtherActor))
        (`/Game/Core/Characters/BP_TopDownCharacter.ApplyEffect` _asbp_top_down_character_3 (`KismetArrayLibrary.Array_Random` (`self.EpicBuffs`)) (`KismetArrayLibrary.Array_Random` (`self.EpicDebuffs`)))
        (`self.K2_DestroyActor`)))))

(event `self.ReceiveTick`
  (params (DeltaSeconds :type "Float (single-precision)"))
  (bind _returnvalue (`GameplayStatics.GetPlayerCharacter` 0))
  (if (and (`KismetSystemLibrary.IsValid` _returnvalue) (`self.isAttrached`))
    (`self.K2_SetActorLocation` (`KismetMathLibrary.VInterpTo` (`self.K2_GetActorLocation`) (`self.K2_GetActorLocation` _returnvalue) DeltaSeconds 2.0))))

(fn `UserConstructionScript`)