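; Player controller that routes Enhanced Input to the controlled BP_TopDownCharacter and lets debuffs change the control scheme.
; SwitchMapContext clears all mappings and applies the context stored under the debuff name in Maps, with "Standart" applied at BeginPlay.
; Move input passes to MoveAction with its Y and X axes as world X and Y, while shoot input starts and stops firing.
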(event `self.ReceiveBeginPlay`
  (`self.SwitchMapContext` "Standart"))

(event `SwitchMapContext`
  (params (DebufName :type String))
  (bind _returnvalue (subsystem `EnhancedInputLocalPlayerSubsystem`))
  (bind (_value _returnvalue_2) (`BlueprintMapLibrary.Map_Find` (`self.Maps`) DebufName))
  ;[1 1 1] Переключение управления под дебафом
  (`EnhancedInputSubsystemInterface.ClearAllMappings` _returnvalue)
  (if _returnvalue_2
    (`EnhancedInputSubsystemInterface.AddMappingContext` _returnvalue _value 0 (struct))))

(event `EnhancedInput|/Game/Core/Controllers/Input/Actions/IA_Move`
  (params (ActionValue :type "Vector2D Structure") (ElapsedSeconds :type "Float (double-precision)") (TriggeredSeconds :type "Float (double-precision)") (InputAction :type "InputAction Object Reference" :default "/Game/Core/Controllers/Input/Actions/IA_Move.IA_Move"))
  (bind (_x _y) (`KismetMathLibrary.BreakVector2D` ActionValue))
  ;[1 1 1] Move
  (:`Triggered`
    (bind _asbp_top_down_character (cast `/Game/Core/Characters/BP_TopDownCharacter` (`self.K2_GetPawn`)))
    (`/Game/Core/Characters/BP_TopDownCharacter.MoveAction` _asbp_top_down_character _y _x)))

(event `EnhancedInput|/Game/Core/Controllers/Input/Actions/IA_Shoot`
  (params (ActionValue :type Boolean) (ElapsedSeconds :type "Float (double-precision)") (TriggeredSeconds :type "Float (double-precision)") (InputAction :type "InputAction Object Reference" :default "/Game/Core/Controllers/Input/Actions/IA_Shoot.IA_Shoot"))
  (bind _returnvalue (`self.K2_GetPawn`))
  (:`Triggered`
    (bind _asbp_top_down_character (cast `/Game/Core/Characters/BP_TopDownCharacter` _returnvalue))
    (`XYZ_GameJam_ProjectCharacter.StartFire` _asbp_top_down_character))
  (:`Completed`
    (bind _asbp_top_down_character_2 (cast `/Game/Core/Characters/BP_TopDownCharacter` _returnvalue))
    (`XYZ_GameJam_ProjectCharacter.StopFire` _asbp_top_down_character_2)))

(fn `UserConstructionScript`)