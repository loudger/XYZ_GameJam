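; Base enemy character Blueprint that handles health, melee attacks, a speed-based dash and death by destroying the actor.
; BeginPlay fills health and sets walk speed, which DashStart raises and EndDash or BreakDash restores.
; DealMeeleDamage re-calls itself after a delay to hit its target repeatedly while CanDamage holds.
; TakeDamage's branches look inverted: non-lethal hits set IsDead and call Death, while lethal hits only subtract health.
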(event `self.ReceiveBeginPlay`
  ;[1 1 1] Установить значение HP
  (set `self.CurrentHealth` (`self.MaxHealth`))
  (set `CharacterMovementComponent.MaxWalkSpeed` (`self.InitialMoveSpeed`) (`self.CharacterMovement`)))

(event `EndDash`
  (set `CharacterMovementComponent.MaxWalkSpeed` (`self.InitialMoveSpeed`) (`self.CharacterMovement`)))

(event `self.ReceiveTick`
  (params (DeltaSeconds :type "Float (single-precision)")))

(event `DashStart`
  (set `CharacterMovementComponent.MaxWalkSpeed` (`self.DashSpeed`) (`self.CharacterMovement`)))

(event `TakeDamage`
  (params (DamageValue :type "Float (double-precision)"))
  (bind _returnvalue (- (`self.CurrentHealth`) DamageValue))
  ;[1 1 1] Получение урона
  (if (<= _returnvalue 0.0)
    (set `self.IsDead` false)
    (set `self.CurrentHealth` _returnvalue)
    (else
      (set `self.IsDead` true)
      (`self.Death`))))

(event `Death`
  ;[1 0 0] DEATH
  (`self.K2_DestroyActor`))

(event `DealMeeleDamage`
  (params (TargetCharacter :type "/Game/Core/Characters/BP_TopDownCharacter Object Reference"))
  ;[0 0.0615 1] Meele Attack
  (if (`self.CanDamage`)
    (`KismetSystemLibrary.Delay` (/ (`self.AttackPerSecond`) 60.0))
    (`/Game/Core/Characters/BP_TopDownCharacter.TakeDamage` TargetCharacter (`self.MeeleDamage`))
    (`self.DealMeeleDamage` TargetCharacter)))

(fn `BreakDash`
  (`self.EndDash`))

(fn `UserConstructionScript`)