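; BP_Barrel is an explosive barrel that deals radial damage to enemies and the player when it dies.
; Death destroys the actor, then calls ExplosionEnemies and ExplosionPerson, two near-identical passes for BP_BaseEnemy and BP_TopDownCharacter, the latter marked as a quick workaround.
; Each pass runs a class-filtered sphere overlap at the barrel's location, draws a debug sphere and applies ExplosionDamage through TakeDamage.
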(event `ExplosionEnemies`
  (bind _returnvalue (`self.K2_GetActorLocation`))
  (bind _explosionradius (`self.ExplosionRadius`))
  ;[1 1 1] Взрыв и нанесение урона вокруг врагам
  (bind _outactors (`KismetSystemLibrary.SphereOverlapActors` _returnvalue _explosionradius (`self.Object TypesExplosion`) "/Game/Core/Enemies/BP_BaseEnemy.BP_BaseEnemy_C"))
  (`KismetSystemLibrary.DrawDebugSphere` _returnvalue _explosionradius 9 (struct :`R` 1.0 :`B` 0.21596 :`A` 1.0) 5.0 0.5)
  (for _array_element _outactors
    (bind _asbp_base_enemy (cast `/Game/Core/Enemies/BP_BaseEnemy` _array_element))
    (`self.TakeDamage` _asbp_base_enemy (`self.ExplosionDamage`))))

(event `ExplosionPerson`
  (bind _returnvalue (`self.K2_GetActorLocation`))
  (bind _explosionradius (`self.ExplosionRadius`))
  ;[1 1 1] Взрыв и нанесение урона вокруг персонажу (Костыль, но так быстрее)
  (bind _outactors (`KismetSystemLibrary.SphereOverlapActors` _returnvalue _explosionradius (`self.Object TypesExplosion`) "/Game/Core/Characters/BP_TopDownCharacter.BP_TopDownCharacter_C"))
  (`KismetSystemLibrary.DrawDebugSphere` _returnvalue _explosionradius 9 (struct :`R` 1.0 :`B` 0.21596 :`A` 1.0) 5.0 0.5)
  (for _array_element _outactors
    (bind _asbp_top_down_character (cast `/Game/Core/Characters/BP_TopDownCharacter` _array_element))
    (`/Game/Core/Characters/BP_TopDownCharacter.TakeDamage` _asbp_top_down_character (`self.ExplosionDamage`))))

(event `self.Death`
  ;[1 1 1] События при смерти
  (`self.K2_DestroyActor`)
  (`self.ExplosionEnemies`)
  (`self.ExplosionPerson`))

(fn `UserConstructionScript`)