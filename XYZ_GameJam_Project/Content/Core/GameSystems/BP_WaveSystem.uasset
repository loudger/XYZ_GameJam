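; BP_WaveSystem is a trigger-box enemy wave spawner that fires when BP_TopDownCharacter overlaps it.
; On BeginPlay it splits the total enemy count into close and far groups using the skeleton combat percentage.
; Each wave spawns the close group at random close spawners, then, after a delay, the far group at far spawners.
; In hard mode, a timer chains further waves until the wave counter runs out.
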(event `self.ReceiveBeginPlay`
  (`self.CalculateEnemy`))

(event `SpawnWave`
  (bind _farspawners (`self.FarSpawners`))
  (bind _closespawners (`self.CloseSpawners`))
  (for _ (range 1 (+ (`self.CloseEnemyNum`) 1))
    (`/Game/Core/GameSystems/BP_EnemySpawner.SpawnEnemy` (`|GetArrayItem` _closespawners (`KismetMathLibrary.RandomIntegerInRange` 0 (`KismetArrayLibrary.Array_LastIndex` _closespawners)))))
  (`KismetSystemLibrary.Delay` (`self.TameBeetwenEnemySpawn`))
  (for _ (range 1 (+ (`self.FarEnemyNum`) 1))
    (`/Game/Core/GameSystems/BP_EnemySpawner.SpawnEnemy` (`|GetArrayItem` _farspawners (`KismetMathLibrary.RandomIntegerInRange` 0 (`KismetArrayLibrary.Array_LastIndex` _farspawners)))))
  (set `self.WaveCounter` (- (`self.WaveCounter`) 1))
  (if (<= (`self.WaveCounter`) 0)
    _
    (elif (`self.HardMode`)
      (`KismetSystemLibrary.K2_SetTimerDelegate` (delegate `HardModeWaveSpawn`) (`self.DelayTimeBeetwenWaves`)))))

(event `self.Box.OnComponentBeginOverlap`
  (params (OverlappedComponent :type "PrimitiveComponent Object Reference") (OtherActor :type "Actor Object Reference") (OtherComp :type "PrimitiveComponent Object Reference") (OtherBodyIndex :type Integer) (bFromSweep :type Boolean) (SweepResult :type "HitResult Structure (by ref)"))
  (cast `/Game/Core/Characters/BP_TopDownCharacter` OtherActor)
  (`self.SpawnWave`))

(event `HardModeWaveSpawn`
  (`self.SpawnWave`))

(fn `CalculateEnemy`
  (bind _output_get (set `self.CloseEnemyNum` (`KismetMathLibrary.Round` (* (/ (`self.PercentSkeletonCombat`) 100.0) (`self.TotalEnemyNum`)))))
  (set `self.FarEnemyNum` (- (`self.TotalEnemyNum`) _output_get)))

(fn `UserConstructionScript`)