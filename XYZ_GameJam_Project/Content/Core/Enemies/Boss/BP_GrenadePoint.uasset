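; Boss grenade impact point that grows a flat area indicator, then explodes and damages player characters inside it.
; On BeginPlay, a Delay loop widens the Void component in X/Y for a set number of steps.
; ExploseEffect then hides Void, destroys the Grenade actor, spawns the particle effect and destroys itself after a short delay.
; Top-down characters overlapping Void take GrenadeDamage at detonation; the ExploseGrenade event is empty.
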(event `ExploseEffect`
  (`SceneComponent.SetVisibility` (`self.Void`) false false)
  (`self.K2_DestroyActor` (`self.Grenade`))
  (`GameplayStatics.SpawnEmitterAtLocation` (`self.Explose Effect`) (`SceneComponent.K2_GetComponentLocation` (`self.Void`)))
  (`KismetSystemLibrary.Delay` 1.0)
  (`self.K2_DestroyActor`))

(event `ScaleVoid`
  (bind _void (`self.Void`))
  (bind (_relativescale3d_x _relativescale3d_y) (`KismetMathLibrary.BreakVector` (`SceneComponent.RelativeScale3D` _void)))
  (`SceneComponent.SetRelativeScale3D` _void (`KismetMathLibrary.MakeVector` (+ _relativescale3d_x 0.05) (+ _relativescale3d_y 0.05)) :!label _label)
  (`KismetSystemLibrary.Delay` (/ (`self.TimeForScale`) 60.0))
  (`/Engine/EditorBlueprintResources/StandardMacros.IncrementInt` (`self.CurrentIterration`)
    (:`  `
      (if (< (`self.CurrentIterration`) (`self.ScaleIterration`))
        (goto _label)
        (else
          (`self.ExploseEffect`)
          (for _array_element (`PrimitiveComponent.GetOverlappingActors` (`self.Void`) "/Game/Core/Characters/BP_TopDownCharacter.BP_TopDownCharacter_C")
            (bind _asbp_top_down_character (cast `/Game/Core/Characters/BP_TopDownCharacter` _array_element))
            (`/Game/Core/Characters/BP_TopDownCharacter.TakeDamage` _asbp_top_down_character (`self.GrenadeDamage`))))))))

(event `self.ReceiveBeginPlay`
  (`self.ScaleVoid`))

(event `ExploseGrenade`)

(fn `UserConstructionScript`)