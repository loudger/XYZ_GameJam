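; AI controller for the close-combat skeleton enemy that chases a target player, attacks in melee and can dash.
; Each tick it either moves toward TargetPlayer or, within attack range, enables CanDamage and deals melee damage through the BP_BaseEnemy pawn.
; While BlockDash is true, it starts the pawn's dash inside a distance band and ends it outside.
; BreakDash, which sets BlockDash at close range, is disconnected from execution.
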(event `self.ReceiveTick`
  (params (DeltaSeconds :type "Float (single-precision)"))
  (`self.MoveOrDamage`)
  (if (`self.BlockDash`)
    (`self.Dash`)))

(fn `AttackPlayer`
  (bind _asbp_top_down_character (cast `/Game/Core/Characters/BP_TopDownCharacter` (`self.TargetPlayer`)))
  (bind _asbp_base_enemy (cast `/Game/Core/Enemies/BP_BaseEnemy` (`self.K2_GetPawn`)))
  (`/Game/Core/Enemies/BP_BaseEnemy.DealMeeleDamage` _asbp_base_enemy _asbp_top_down_character))

(fn `BreakDash`
  (if (<= (`self.GetDistanceTo` (`self.K2_GetPawn`) (`self.TargetPlayer`)) 50.0)
    (set `self.BlockDash` true)
    (bind _asbp_base_enemy (cast `/Game/Core/Enemies/BP_BaseEnemy` (`self.K2_GetPawn`)))
    (`/Game/Core/Enemies/BP_BaseEnemy.BreakDash` _asbp_base_enemy)))

(fn `Dash`
  (if (and (<= (`self.GetDistanceTo` (`self.K2_GetPawn`) (`self.TargetPlayer`)) (`self.DashDistance`)) (> (`self.GetDistanceTo` (`self.K2_GetPawn`) (`self.TargetPlayer`)) 50.0))
    (bind _asbp_base_enemy (cast `/Game/Core/Enemies/BP_BaseEnemy` (`self.K2_GetPawn`))
      (:`then`
        (`/Game/Core/Enemies/BP_BaseEnemy.DashStart` _asbp_base_enemy))
      (:`CastFailed`
        (`KismetSystemLibrary.PrintString` "Hello")))
    (else
      (bind _asbp_base_enemy_2 (cast `/Game/Core/Enemies/BP_BaseEnemy` (`self.K2_GetPawn`)))
      (`/Game/Core/Enemies/BP_BaseEnemy.EndDash` _asbp_base_enemy_2))))

(fn `MoveOrDamage`
  (if (< (`self.GetDistanceTo` (`self.K2_GetPawn`) (`self.TargetPlayer`)) (`self.MinimalDistanceForAttack`))
    (bind _asbp_base_enemy (cast `/Game/Core/Enemies/BP_BaseEnemy` (`self.K2_GetPawn`)))
    (set `/Game/Core/Enemies/BP_BaseEnemy.CanDamage` true _asbp_base_enemy)
    (`self.AttackPlayer`)
    (else
      (bind _asbp_base_enemy_2 (cast `/Game/Core/Enemies/BP_BaseEnemy` (`self.K2_GetPawn`)))
      (set `/Game/Core/Enemies/BP_BaseEnemy.CanDamage` false _asbp_base_enemy_2)
      (`self.MoveToPlayer` self (`self.TargetPlayer`)))))

(fn `MoveToPlayer`
  (params (Controller :type "Controller Object Reference") (Goal :type "Actor Object Reference"))
  (locals (CashedOwner :type "/Game/Core/Enemies/BP_BaseEnemy Object Reference"))
  (set `self.TargetPlayer` Goal)
  (`AIBlueprintHelperLibrary.SimpleMoveToActor` self Goal))

(fn `UserConstructionScript`)